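; BP_FireParrent12 is an interactable fire hazard, apparently a parent class, with placeholder interaction functions and debug prints.
; Overlapping its sphere as the first-person character enables interaction and shows a widget, hidden again on exit.
; StartFire, not invoked by live logic here, randomizes a timer; a self-calling delayed event counts it down to a death message.
; Delayed Tick reveals the fire sphere once the timer drops below half.
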(event `self.ReceiveBeginPlay`
  ; Interaction Temp
)

(event `self.SphereCollision.OnComponentBeginOverlap`
  (params (OverlappedComponent :type "PrimitiveComponent Object Reference") (OtherActor :type "Actor Object Reference") (OtherComp :type "PrimitiveComponent Object Reference") (OtherBodyIndex :type Integer) (bFromSweep :type Boolean) (SweepResult :type "HitResult Structure (by ref)"))
  ; Interaction Zone
  (cast `/Game/65070201/BP/BP_FirstPersonCharacterNew` OtherActor)
  (set `self.CanInteract` true)
  (if (`self.CanInteract`)
    (`SceneComponent.SetVisibility` (`self.Widget`) true false)
    (`KismetSystemLibrary.PrintString` "enter")))

(event `self.SphereCollision.OnComponentEndOverlap`
  (params (OverlappedComponent :type "PrimitiveComponent Object Reference") (OtherActor :type "Actor Object Reference") (OtherComp :type "PrimitiveComponent Object Reference") (OtherBodyIndex :type Integer))
  ; Interaction Zone
  (set `self.CanInteract` false)
  (`SceneComponent.SetVisibility` (`self.Widget`) false false)
  (`KismetSystemLibrary.PrintString` "leave"))

(event `self.ReceiveTick`
  (params (DeltaSeconds :type "Float (single-precision)"))
  ; Interact Condition
  (`KismetSystemLibrary.Delay` 1.0)
  (`KismetSystemLibrary.PrintString` (`KismetStringLibrary.Conv_DoubleToString` (`self.Timer`)))
  (if (< (`self.Timer`) (`self.ConditionTimer`))
    (`SceneComponent.SetVisibility` (`self.Sphere`) true false)
    (set `self.OnFire` true)
    (set `self.CanInteract` true)))

(event `StartFire`
  ; Fire Starter
  (bind _output_get (set `self.Timer` (`KismetMathLibrary.RandomFloatInRange` 20.0 60.0)))
  (set `self.ConditionTimer` (/ _output_get 2.0)))

(event `decreaseTimer`
  (bind _timer (`self.Timer`))
  ; Timer
  (if (> _timer 0.0)
    (`KismetSystemLibrary.Delay` 1.0)
    (bind _result (`/Engine/EditorBlueprintResources/StandardMacros.DecrementFloat` _timer)
      (:`  `
        (set `self.Timer` _result)
        (`self.decreaseTimer`)))
    (else
      (`KismetSystemLibrary.PrintString` "u r  ded"))))

(fn `CanIteractWithItem`
  (returns (CheckItemResult :type Boolean))
  (return false))

(fn `CheckItem`)

(fn `OnInteract`
  (return))

(fn `UserConstructionScript`)