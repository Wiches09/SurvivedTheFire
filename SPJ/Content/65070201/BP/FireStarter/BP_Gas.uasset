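; BP_Gas is a child fire hazard the player puts out using the held item.
; On BeginPlay it sets its correct item, calls the player's Interact, then starts the fire and timer through an always-true branch.
; OnInteract accepts the matching item and shows the lose widget for a wrong one.
; CheckItem separately tests a different hardcoded item, hiding the sphere and clearing the fire flags before calling StartFire again.
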(event `self.ReceiveBeginPlay`
  (`parent.ReceiveBeginPlay`)
  (set `self.CorrectItem` "Item2 Cube")
  (bind _asbp_first_person_character_new (cast `/Game/65070201/BP/BP_FirstPersonCharacterNew` (`GameplayStatics.GetPlayerCharacter` 0)))
  (`/Game/65070201/BP/BP_FirstPersonCharacterNew.Interact` _asbp_first_person_character_new)
  (if true
    (`KismetSystemLibrary.PrintString` "PutOutFire")
    (`self.StartFire`)
    (`self.decreaseTimer`)
    (else
      (`KismetSystemLibrary.PrintString` "You died"))))

(fn `CheckItem`
  (locals (TrueItem :type Name))
  (`parent.CheckItem`)
  (`KismetSystemLibrary.PrintString` "------------------")
  (bind _asbp_first_person_character_new (cast `/Game/65070201/BP/BP_FirstPersonCharacterNew` (`GameplayStatics.GetPlayerCharacter` 0)))
  (set `self.PlayerCurrentItem` (`/Game/65070201/BP/BP_FirstPersonCharacterNew.CurrentItem` _asbp_first_person_character_new))
  (`KismetSystemLibrary.PrintString` "---------------")
  (`KismetSystemLibrary.PrintString` "in checkitem")
  (set `local.TrueItem` "Item 1 Ball")
  (if (== (`self.PlayerCurrentItem`) (`local.TrueItem`))
    (`KismetSystemLibrary.PrintString` "Fire is gone!")
    (`SceneComponent.SetVisibility` (`self.Sphere`) false false)
    (set `self.OnFire` false)
    (set `self.CanInteract` false)
    (`self.StartFire`)
    (else
      (`KismetSystemLibrary.PrintString` "You Lose!"))))

(fn `OnInteract`
  (returns (canInteract :type Boolean))
  (`parent.OnInteract`)
  (`KismetSystemLibrary.PrintString` "in chld")
  (bind _asbp_first_person_character_new (cast `/Game/65070201/BP/BP_FirstPersonCharacterNew` (`GameplayStatics.GetPlayerCharacter` 0)))
  (bind _currentitem (`/Game/65070201/BP/BP_FirstPersonCharacterNew.CurrentItem` _asbp_first_person_character_new))
  (if (== (`self.CorrectItem`) _currentitem)
    (`KismetSystemLibrary.PrintString` "correctItem")
    (return true)
    (elif (== _currentitem "None")
      (`KismetSystemLibrary.PrintString` "No Item in your han d")
      (else
        (`KismetSystemLibrary.PrintString` "WrongItem")
        (bind _returnvalue (`|CreateWidget` "/Game/65070201/Widget/W_Lose.W_Lose_C"))
        (`UserWidget.AddToViewport` _returnvalue 0)
        (return false)))))

(fn `UserConstructionScript`
  (`parent.UserConstructionScript`))