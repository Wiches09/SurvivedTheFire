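; BP_Cloth is a cloth item Blueprint that can change from dry to wet.
; Its ChangeDryToWet override calls the parent, caches the first-person player character and reads that character's current item.
; If the held item has a specific ItemType, the cloth switches its own ItemType; otherwise it prints that the cloth is already wet.
; The event graph holds only disabled stubs, and NewFunction_0 is empty.
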(fn `ChangeDryToWet`
  (locals (Player :type "/Game/65070201/BP/BP_FirstPersonCharacterNew Object Reference"))
  (`parent.ChangeDryToWet`)
  (bind _asbp_first_person_character_new (cast `/Game/65070201/BP/BP_FirstPersonCharacterNew` (`GameplayStatics.GetPlayerCharacter` 0)))
  (bind _output_get (set `local.Player` _asbp_first_person_character_new))
  (bind _output_get_2 (set `self.HoldingItem` (`/Game/65070201/BP/BP_FirstPersonCharacterNew.CurrentItem` _output_get)))
  (if (`|EnumEquality` (`.ItemType_8_1537EF594B6356EB84330E9633A8CB5B` (break `/Game/65070201/BP/ItemDetails` _output_get_2)) "NewEnumerator3")
    (set `self.ItemType` "NewEnumerator0")
    (else
      (`KismetSystemLibrary.PrintString` "Cloth is already WET" true true (struct :`R` 0.02168 :`G` 1.0 :`A` 1.0)))))

(fn `NewFunction_0`)

(fn `UserConstructionScript`
  (`parent.UserConstructionScript`))