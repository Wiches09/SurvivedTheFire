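; BP_NewPlugFire is an interactable plug fire hazard that recurs on a randomized timer and triggers game over if left too long.
; A self-recalling one-second countdown drives it, and Tick shows the fire and enables interaction below half time.
; Inside the box, player interaction with a full water bucket while the breaker is off restarts the cycle, empties the bucket and resets the breaker flag.
; At zero, W_GameOver appears with UI-only input.
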(event `self.ReceiveBeginPlay`
  (`self.StartFire`)
  (`self.decreaseTimer`))

(event `self.Box.OnComponentEndOverlap`
  (params (OverlappedComponent :type "PrimitiveComponent Object Reference") (OtherActor :type "Actor Object Reference") (OtherComp :type "PrimitiveComponent Object Reference") (OtherBodyIndex :type Integer))
  ; Interaction
  (set `self.IsInRange` false))

(event `self.Box.OnComponentBeginOverlap`
  (params (OverlappedComponent :type "PrimitiveComponent Object Reference") (OtherActor :type "Actor Object Reference") (OtherComp :type "PrimitiveComponent Object Reference") (OtherBodyIndex :type Integer) (bFromSweep :type Boolean) (SweepResult :type "HitResult Structure (by ref)"))
  ; Interaction
  (set `self.IsInRange` true)
  (bind _asbp_first_person_character_new (cast `/Game/65070201/BP/BP_FirstPersonCharacterNew` (`GameplayStatics.GetPlayerCharacter` 0)))
  (bind _output_get (set `self.PlayerRef` _asbp_first_person_character_new))
  (add `/Game/65070201/BP/BP_FirstPersonCharacterNew.Interaction` _output_get (delegate `Interact`)))

(event `Interact`
  ; Interaction
  (if (`self.IsInRange`)
    (if (`self.CanInteract`)
      (if (`self.IsBreakerOff`)
        (if (`KismetStringLibrary.EqualEqual_StrStr` (`/Game/65070201/BP/BP_FirstPersonCharacterNew.CurrentItemName` (`self.PlayerRef`)) "Water Bucket")
          (`KismetSystemLibrary.PrintString` "true")
          (if (`/Game/65070201/BP/BP_FirstPersonCharacterNew.IsBucketFull` (`self.PlayerRef`))
            (`self.StartFire`)
            (else
              (`KismetSystemLibrary.PrintString` "Not Wet")))
          (else
            (`KismetSystemLibrary.PrintString` "false")))
        (else
          (`KismetSystemLibrary.PrintString` "breaker still on"))))))

(event `self.ReceiveTick`
  (params (DeltaSeconds :type "Float (single-precision)"))
  ; Interact Condition
  (`KismetSystemLibrary.Delay` 1.0)
  (`KismetSystemLibrary.PrintString` (`KismetStringLibrary.Concat_StrStr` "Plugfire: " (`KismetStringLibrary.Conv_DoubleToString` (`self.Timer`))))
  (if (< (`self.Timer`) (`self.ConditionTimer`))
    (`SceneComponent.SetVisibility` (`self.fire`) true false)
    (set `self.OnFire` true)
    (set `self.CanInteract` true)))

(event `StartFire`
  (bind _playerref (`self.PlayerRef`))
  ; Fire Starter
  (bind _output_get (set `self.Timer` (`KismetMathLibrary.RandomFloatInRange` 20.0 60.0)))
  (set `self.ConditionTimer` (/ _output_get 2.0))
  (set `self.OnFire` false)
  (set `self.CanInteract` false)
  (`SceneComponent.SetVisibility` (`self.fire`) false false)
  (`KismetSystemLibrary.PrintString` "started new fire")
  (set `self.IsBreakerOff` false)
  (set `/Game/65070201/BP/BP_FirstPersonCharacterNew.IsBucketFull` false _playerref)
  (set `/Game/65070201/BP/BP_FirstPersonCharacterNew.CurrentBucketMesh` (`/Game/65070201/BP/BP_FirstPersonCharacterNew.BucketMeshDry` _playerref) _playerref))

(event `decreaseTimer`
  (bind _returnvalue (`GameplayStatics.GetPlayerController` 0))
  (bind _timer (`self.Timer`))
  ; Timer
  (if (> _timer 0.0)
    (`KismetSystemLibrary.Delay` 1.0)
    (bind _result (`/Engine/EditorBlueprintResources/StandardMacros.DecrementFloat` _timer)
      (:`  `
        (set `self.Timer` _result)
        (`self.decreaseTimer`)))
    (else
      (`KismetSystemLibrary.PrintString` "u r  ded")
      (bind _returnvalue_2 (`|CreateWidget` "/Game/MyBP/Widget/W_GameOver.W_GameOver_C"))
      (`UserWidget.AddToViewport` _returnvalue_2 0)
      (`WidgetBlueprintLibrary.SetInputMode_UIOnlyEx` _returnvalue null)
      (set `PlayerController.bShowMouseCursor` true _returnvalue))))

(fn `UserConstructionScript`)