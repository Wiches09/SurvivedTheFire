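; Base fire hazard interactable that runs a random countdown and shows the lose screen when it reaches zero.
; Below half time it shows its sphere as on fire and becomes interactable; StartFire rerolls the timer and hides it.
; An overlap sphere toggles the prompt widget, and Interact registers the actor as the first-person character's interaction target.
; CheckItem, OnInteract and CanIteractWithItem are empty stubs, and debug prints remain throughout.
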(event `self.ReceiveBeginPlay`
  ; Interaction Temp
  (bind _asbp_first_person_character_new (cast `/Game/65070201/BP/BP_FirstPersonCharacterNew` (`GameplayStatics.GetPlayerCharacter` 0))
    (:`then`
      (`KismetSystemLibrary.PrintText` "success")
      (add `/Game/65070201/BP/BP_FirstPersonCharacterNew.Interaction` _asbp_first_person_character_new (`|CreateDelegate` :!event `Interact`))
      (bind _output_get (set `self.Timer` (`KismetMathLibrary.RandomFloatInRange` 10.0 20.0)))
      (set `self.ConditionTimer` (/ _output_get 2.0))
      (`self.decreaseTimer`))
    (:`CastFailed`
      (`KismetSystemLibrary.PrintText` "fail"))))

(event `self.SphereCollision.OnComponentBeginOverlap`
  (params (OverlappedComponent :type "PrimitiveComponent Object Reference") (OtherActor :type "Actor Object Reference") (OtherComp :type "PrimitiveComponent Object Reference") (OtherBodyIndex :type Integer) (bFromSweep :type Boolean) (SweepResult :type "HitResult Structure (by ref)"))
  ; Interaction Zone
  (cast `/Game/65070201/BP/BP_FirstPersonCharacterNew` OtherActor)
  (set `self.CanInteract` true)
  (if (`self.CanInteract`)
    (`SceneComponent.SetVisibility` (`self.Widget`) true false)
    (`KismetSystemLibrary.PrintString` "enter")))

(event `self.SphereCollision.OnComponentEndOverlap`
  (params (OverlappedComponent :type "PrimitiveComponent Object Reference") (OtherActor :type "Actor Object Reference") (OtherComp :type "PrimitiveComponent Object Reference") (OtherBodyIndex :type Integer))
  ; Interaction Zone
  (set `self.CanInteract` false)
  (`SceneComponent.SetVisibility` (`self.Widget`) false false)
  (`KismetSystemLibrary.PrintString` "leave"))

(event `self.ReceiveTick`
  (params (DeltaSeconds :type "Float (single-precision)"))
  ; Interact Condition
  (`KismetSystemLibrary.Delay` 1.0)
  (`KismetSystemLibrary.PrintString` (`KismetStringLibrary.Conv_DoubleToString` (`self.Timer`)))
  (if (< (`self.Timer`) (`self.ConditionTimer`))
    (`SceneComponent.SetVisibility` (`self.Sphere`) true false)
    (set `self.OnFire` true)
    (set `self.CanInteract` true)))

(event `StartFire`
  ; Fire Starter
  (bind _output_get (set `self.Timer` (`KismetMathLibrary.RandomFloatInRange` 20.0 60.0)))
  (set `self.ConditionTimer` (/ _output_get 2.0))
  (set `self.OnFire` false)
  (set `self.CanInteract` false)
  (`SceneComponent.SetVisibility` (`self.Sphere`) false false)
  (`KismetSystemLibrary.PrintString` "started new fire"))

(event `decreaseTimer`
  (bind _returnvalue (`GameplayStatics.GetPlayerController` 0))
  (bind _timer (`self.Timer`))
  ; Timer
  (if (> _timer 0.0)
    (`KismetSystemLibrary.Delay` 1.0)
    (bind _result (`/Engine/EditorBlueprintResources/StandardMacros.DecrementFloat` _timer)
      (:`  `
        (set `self.Timer` _result)
        (`self.decreaseTimer`)))
    (else
      (`KismetSystemLibrary.PrintString` "u r  ded")
      (bind _returnvalue_2 (`|CreateWidget` "/Game/65070201/Widget/W_Lose.W_Lose_C"))
      (`UserWidget.AddToViewport` _returnvalue_2 0)
      (`WidgetBlueprintLibrary.SetInputMode_UIOnlyEx` _returnvalue null)
      (set `PlayerController.bShowMouseCursor` true _returnvalue))))

(event `Interact`
  (if (`self.CanInteract`)
    (bind _asbp_first_person_character_new (cast `/Game/65070201/BP/BP_FirstPersonCharacterNew` (`GameplayStatics.GetPlayerCharacter` 0)))
    (set `/Game/65070201/BP/BP_FirstPersonCharacterNew.CurrentInteractionTo` self _asbp_first_person_character_new)))

(fn `CanIteractWithItem`
  (returns (CheckItemResult :type Boolean))
  (return false))

(fn `CheckItem`)

(fn `OnInteract`
  (returns (canInteract :type Boolean))
  (return false))

(fn `UserConstructionScript`)