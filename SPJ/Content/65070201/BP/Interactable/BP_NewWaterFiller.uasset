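; BP_NewWaterFiller is an interactable water source that wets the player's cloth or fills their bucket.
; Box overlap events toggle an in-range flag, and overlap begin caches the first-person character and binds Interact to its interaction event.
; When triggered in range, Interact sets the player's wet-cloth flag if the current item is named Cloth, otherwise the full-bucket flag, and prints the result.
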(event `self.Box.OnComponentEndOverlap`
  (params (OverlappedComponent :type "PrimitiveComponent Object Reference") (OtherActor :type "Actor Object Reference") (OtherComp :type "PrimitiveComponent Object Reference") (OtherBodyIndex :type Integer))
  ; Interact
  (set `self.IsInRange` false))

(event `self.Box.OnComponentBeginOverlap`
  (params (OverlappedComponent :type "PrimitiveComponent Object Reference") (OtherActor :type "Actor Object Reference") (OtherComp :type "PrimitiveComponent Object Reference") (OtherBodyIndex :type Integer) (bFromSweep :type Boolean) (SweepResult :type "HitResult Structure (by ref)"))
  ; Interact
  (set `self.IsInRange` true)
  (bind _asbp_first_person_character_new (cast `/Game/65070201/BP/BP_FirstPersonCharacterNew` (`GameplayStatics.GetPlayerCharacter` 0)))
  (bind _output_get (set `self.PlayerRef` _asbp_first_person_character_new))
  (add `/Game/65070201/BP/BP_FirstPersonCharacterNew.Interaction` _output_get (delegate `Interact`)))

(event `Interact`
  (bind _playerref (`self.PlayerRef`))
  ; Interact
  (if (`self.IsInRange`)
    (if (`KismetStringLibrary.EqualEqual_StrStr` (`/Game/65070201/BP/BP_FirstPersonCharacterNew.CurrentItemName` (`self.PlayerRef`)) "Cloth")
      (`KismetSystemLibrary.PrintString` "cloth is now wet")
      (set `/Game/65070201/BP/BP_FirstPersonCharacterNew.IsClothWet` true _playerref)
      (else
        (`KismetSystemLibrary.PrintString` "bucket is now full")
        (set `/Game/65070201/BP/BP_FirstPersonCharacterNew.IsBucketFull` true _playerref)))))

(fn `UserConstructionScript`)